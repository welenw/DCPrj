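; Base Blueprint for enemies, with an unfinished damage calculation based on typed damage and resistances.
; CalculateDamage sums normal, fire, water, earth and lightning damage, subtracts the summed resistances and only prints the result.
; Resistances offset the total rather than their matching type, and the result is not clamped.
; AnyDamage is empty, and the logic that would reduce and print HealthCurrent is disconnected, so health never changes here.
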(event `self.ReceiveAnyDamage`
  (params (Damage :type "Float (single-precision)") (DamageType :type "DamageType Object Reference") (InstigatedBy :type "Controller Object Reference") (DamageCauser :type "Actor Object Reference")))

(event `CalculateDamage`
  (params (DamageTypes :type "/Game/Blueprints/Structs/Struct_DamageTypes Structure"))
  (bind (_damageresistance_normalresistance _damageresistance_fireresistance _damageresistance_waterresistance _damageresistance_earthresistance _damageresistance_lightningresistance) (break `/Game/Blueprints/Structs/Struct_DamageResistance` (`self.DamageResistance`)))
  (`KismetSystemLibrary.PrintString` (`KismetStringLibrary.Conv_DoubleToString` (- (+ DamageTypes_NormalDamage_16_A7AEE815408D0F738B21C58CCCF8333C DamageTypes_FireDamage_17_7A218AAA475A6A5B70CC7CB563858BC6 DamageTypes_WaterDamage_19_0101FC144ABDEC3A8686CCBF56B096F8 DamageTypes_EarthDamage_20_845952AE45EFB5EC0C0F4AA598BF248B DamageTypes_LightningDamage_21_BEFC74824BCCBF5540862A90CC53B2A4) (+ _damageresistance_normalresistance _damageresistance_fireresistance _damageresistance_waterresistance _damageresistance_earthresistance _damageresistance_lightningresistance)))))

(fn `UserConstructionScript`)