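; Dungeon spawner component for BP_DungeonGenerator that scatters a set quantity of actors across the generated floor at BeginPlay.
; It draws random tiles from room floors, plus corridors unless RoomOnly, retrying any within MinDistance of the previous spawn only.
; The first SpawnList class to pass its weighted roll spawns there, and the tile is removed.
; All rolls use the dungeon's random stream.
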(event `self.ReceiveBeginPlay`
  (`self.TriggerSpawnThings`))

(event `TriggerSpawnThings`
  (bind _dungeon (`self.Dungeon`))
  (bind _floortiles (`/Game/Blueprints/Dungeon/BP_DungeonGenerator.FloorTiles` _dungeon))
  (bind _asbp_dungeon_generator (cast `/Game/Blueprints/Dungeon/BP_DungeonGenerator` (`self.GetOwner`)))
  (set `self.Dungeon` _asbp_dungeon_generator)
  (if (`self.RoomOnly`)
    (set `self.FloorTiles` _floortiles)
    (else
      (set `self.FloorTiles` _floortiles)
      (`KismetArrayLibrary.Array_Append` (`self.FloorTiles`) (`/Game/Blueprints/Dungeon/BP_DungeonGenerator.CorridorTiles` _dungeon))))
  (`self.SpawnItems`))

(fn `SpawnItems`
  (locals (ItemsSpawned :type Integer) (FloorIndex :type Integer) (LastLocation :type "Vector Structure" :default (0.0 0.0 0.0)))
  (bind _dungeon (`self.Dungeon`))
  (bind _spawnlist (`self.SpawnList`))
  (bind _returnvalue (* (`KismetMathLibrary.Conv_IntVectorToVector` (`|GetArrayItem` (`self.FloorTiles`) (`local.FloorIndex`))) (`/Game/Blueprints/Dungeon/BP_DungeonGenerator.Scale` _dungeon)))
  ;[1 1 1] While spawns are less than desired quantity, loops spawn logic
  (while (> (`self.Quantity`) (`local.ItemsSpawned`))
    ;[1 1 1] Get random floor tile, test if minimum distance is respected
    (bind _output_get (set `local.FloorIndex` (`KismetMathLibrary.RandomIntegerInRangeFromStream` 0 (`KismetArrayLibrary.Array_LastIndex` (`self.FloorTiles`)) (`/Game/Blueprints/Dungeon/BP_DungeonGenerator.Stream` (`self.Dungeon`))) :!label _label))
    (if (== (* (`KismetMathLibrary.Conv_IntVectorToVector` (`|GetArrayItem` (`self.FloorTiles`) _output_get)) (`/Game/Blueprints/Dungeon/BP_DungeonGenerator.Scale` (`self.Dungeon`))) (`local.LastLocation`) :`ErrorTolerance` (`self.MinDistance`))
      (goto _label)
      (else
        ;[1 1 1] Loop through spawn list. If item spawn is true stop looping
        (bind _keys (`BlueprintMapLibrary.Map_Keys` _spawnlist))
        (for _array_element _keys
          (if (`KismetMathLibrary.RandomBoolWithWeightFromStream` (`BlueprintMapLibrary.Map_Find` _spawnlist _array_element) (`/Game/Blueprints/Dungeon/BP_DungeonGenerator.Stream` (`self.Dungeon`)))
            (`|ExecutionSequence`
              (:`then_0`
                ;[1 1 1] Spawn actor, save previous location, remove tile from list and increment item spawned counter
                (`|SpawnActorFromClass` _array_element (`KismetMathLibrary.Conv_VectorToTransform` (+ _returnvalue (`Actor.K2_GetActorLocation` _dungeon) (`self.Offset`))) "Undefined" "OverrideRootScale" null null)
                (set `local.LastLocation` _returnvalue)
                (`KismetArrayLibrary.Array_Remove` (`self.FloorTiles`) (`local.FloorIndex`))
                (`/Engine/EditorBlueprintResources/StandardMacros.IncrementInt` (`local.ItemsSpawned`)))
              (:`then_1`
                (break)))))))))