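; Base weapon Blueprint that fires projectiles on behalf of the first-person player character.
; BeginPlay caches player 0's character as the owner reference.
; Shoot spawns the configured projectile at the muzzle, shifted by the player's camera-rotated gun offset and aligned to the camera's rotation.
; The weapon passes its projectile speed, damage types and elemental particle system into each spawned projectile.
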(event `self.ReceiveBeginPlay`
  (bind _asfirst_person_character (cast `/Game/Blueprints/PlayerCharacter/FirstPersonCharacter` (`GameplayStatics.GetPlayerCharacter` 0)))
  (set `self.PlayerReference` _asfirst_person_character))

(fn `Shoot`
  (bind _playerreference (`self.PlayerReference`))
  (bind _returnvalue (`SceneComponent.K2_GetComponentRotation` (`/Game/Blueprints/PlayerCharacter/FirstPersonCharacter.FirstPersonCamera` _playerreference)))
  (`|SpawnActorFromClass` "/Game/Blueprints/Weapons/Projectile.Projectile_C" (`KismetMathLibrary.MakeTransform` (+ (`SceneComponent.K2_GetComponentLocation` (`self.Muzzle`)) (`KismetMathLibrary.GreaterGreater_VectorRotator` (`/Game/Blueprints/PlayerCharacter/FirstPersonCharacter.GunOffset` _playerreference) _returnvalue)) _returnvalue) "Undefined" "OverrideRootScale" null (`self.ProjectileSpeed`) (`self.DamageTypes`) (`self.Element`) null))

(fn `UserConstructionScript`)